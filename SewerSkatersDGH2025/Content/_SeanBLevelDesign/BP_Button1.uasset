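; BP_Button1 is a one-shot level button that moves a linked bridge when something overlaps its box.
; The first overlap calls MoveBridgeWithButton on BridgeSelect and sets IsPressed to block repeats, without filtering the overlapping actor.
; It also increments its own ButtonsPressed and the Buttons counter on player 0's skate character, then plays a sound if that cast succeeds.
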(event `self.Box.OnComponentBeginOverlap`
  (params (OverlappedComponent :type "PrimitiveComponent Object Reference") (OtherActor :type "Actor Object Reference") (OtherComp :type "PrimitiveComponent Object Reference") (OtherBodyIndex :type Integer) (bFromSweep :type Boolean) (SweepResult :type "HitResult Structure (by ref)"))
  (if (not (`self.isPressed`))
    (`/Game/_SeanBLevelDesign/BP_Door1.MoveBridgeWithButton` (`self.BridgeSelect`))
    (set `self.isPressed` true)
    (set `self.buttonsPressed` (+ (`self.buttonsPressed`) 1))
    (bind _asbp_third_person_character_skate (cast `/Game/Assets/Blueprints/BP_ThirdPersonCharacterSkate` (`GameplayStatics.GetPlayerCharacter` 0)))
    (bind _result (`/Engine/EditorBlueprintResources/StandardMacros.IncrementInt` (`/Game/Assets/Blueprints/BP_ThirdPersonCharacterSkate.Buttons` _asbp_third_person_character_skate))
      (:`  `
        (set `/Game/Assets/Blueprints/BP_ThirdPersonCharacterSkate.Buttons` _result _asbp_third_person_character_skate)
        (`AudioComponent.Play` (`self.SFX`) 0.0)))))

(fn `UserConstructionScript`)