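; Points is a cheese pickup that adds to the skateboarder player's score when touched.
; On overlap with an actor tagged Player, it casts the first player character to BP_SkateBoy and increments its Cheese count by one.
; It then hides itself, disables collision, plays a sound and destroys itself after a short delay.
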(event `self.ReceiveBeginPlay`)

(event `self.ReceiveActorBeginOverlap`
  (params (OtherActor :type "Actor Object Reference"))
  (if (`self.ActorHasTag` OtherActor "Player")
    (bind _asbp_skate_boy (cast `/Game/Assets/Blueprints/BP_SkateBoy` (`GameplayStatics.GetPlayerCharacter` 0)))
    (set `/Game/Assets/Blueprints/BP_SkateBoy.Cheese` (+ 1 (`/Game/Assets/Blueprints/BP_SkateBoy.Cheese` _asbp_skate_boy)) _asbp_skate_boy)
    (`self.SetActorHiddenInGame` true)
    (`self.SetActorEnableCollision` false)
    (`AudioComponent.Play` (`self.sfx`) 0.0)
    (`KismetSystemLibrary.Delay` 0.2)
    (`self.K2_DestroyActor`)))

(fn `UserConstructionScript`)