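; WanderingAI is an AI pawn that roams at random until the player runs into it, then gets launched and leaves Points behind.
; RandomRoam loops from BeginPlay, walking slowly to random reachable nearby points and pausing randomly between moves; it repeats only after a successful move.
; A capsule hit from a Player-tagged actor enables physics, disables movement, applies an upward impulse, then after a delay spawns Points and destroys the pawn.
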(event `self.ReceiveBeginPlay`
  (`self.RandomRoam`))

(event `RandomRoam`
  (set `CharacterMovementComponent.MaxWalkSpeed` 150.0 (`self.CharacterMovement`))
  (`|AIMoveTo` self (`NavigationSystemV1.K2_GetRandomReachablePointInRadius` (`self.K2_GetActorLocation`) 1000.0 null null) null
    (:`OnSuccess`
      (`KismetSystemLibrary.Delay` (`KismetMathLibrary.RandomFloatInRange` 1.0 8.0))
      (`self.RandomRoam`))))

(event `self.CapsuleComponent.OnComponentHit`
  (params (HitComponent :type "PrimitiveComponent Object Reference") (OtherActor :type "Actor Object Reference") (OtherComp :type "PrimitiveComponent Object Reference") (NormalImpulse :type "Vector Structure") (Hit :type "HitResult Structure (by ref)"))
  (if (`self.ActorHasTag` OtherActor "Player")
    (cast `/Game/Assets/Blueprints/BP_ThirdPersonCharacterSkate` (`GameplayStatics.GetPlayerCharacter` 0))
    (`PrimitiveComponent.SetSimulatePhysics` (`self.CapsuleComponent`) true)
    (`CharacterMovementComponent.DisableMovement` (`self.CharacterMovement`))
    (`PrimitiveComponent.AddImpulse` (`self.CapsuleComponent`) (0.0 0.0 1000.0) "None" false)
    (`KismetSystemLibrary.Delay` 2.0)
    (`|SpawnActorFromClass` "/Game/Assets/Blueprints/Points.Points_C" (`self.GetTransform`) "Undefined" "MultiplyWithRoot" null null)
    (`self.K2_DestroyActor`)))

(fn `UserConstructionScript`)