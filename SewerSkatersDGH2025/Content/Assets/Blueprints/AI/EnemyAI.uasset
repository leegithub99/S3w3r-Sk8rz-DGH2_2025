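; Enemy AI character that patrols, chases pawns it sees and is knocked out when the skateboarding player hits it.
; It walks between four looping patrol points with random pauses, then speeds up to chase on PawnSensing sightings.
; A retriggerable delay returns it to patrol once sightings stop for a few seconds.
; A player capsule hit switches on physics, launches it upward, then replaces it with a Points actor after a delay.
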(event `self.ReceiveBeginPlay`
  (`self.Patrolling`))

(event `Patrolling`
  (set `CharacterMovementComponent.MaxWalkSpeed` 200.0 (`self.CharacterMovement`))
  (`|AIMoveTo` self (`|GetArrayItem` (`self.PatrolPoints`) (`self.Locations`)) null
    (:`OnSuccess`
      (`KismetSystemLibrary.Delay` (`KismetMathLibrary.RandomFloatInRange` 1.0 3.0))
      (`self.Patrolling`)
      (`/Engine/EditorBlueprintResources/StandardMacros.IncrementInt` (`self.Locations`)
        (:`  `
          (if (== (`self.Locations`) 4)
            (set `self.Locations` 0)))))))

(event `self.PawnSensing.OnSeePawn`
  (params (Pawn :type "Pawn Object Reference"))
  (set `CharacterMovementComponent.MaxWalkSpeed` 500.0 (`self.CharacterMovement`))
  (`|ExecutionSequence`
    (:`then_0`
      (`|AIMoveTo` self (0.0 0.0 0.0) Pawn))
    (:`then_1`
      (`KismetSystemLibrary.RetriggerableDelay` 3.0)
      (`self.Patrolling`))))

(event `self.CapsuleComponent.OnComponentHit`
  (params (HitComponent :type "PrimitiveComponent Object Reference") (OtherActor :type "Actor Object Reference") (OtherComp :type "PrimitiveComponent Object Reference") (NormalImpulse :type "Vector Structure") (Hit :type "HitResult Structure (by ref)"))
  (if (`self.ActorHasTag` OtherActor "Player")
    (cast `/Game/Assets/Blueprints/BP_ThirdPersonCharacterSkate` (`GameplayStatics.GetPlayerCharacter` 0))
    (`PrimitiveComponent.SetSimulatePhysics` (`self.CapsuleComponent`) true)
    (`CharacterMovementComponent.DisableMovement` (`self.CharacterMovement`))
    (`PrimitiveComponent.AddImpulse` (`self.CapsuleComponent`) (0.0 0.0 1000.0) "None" false)
    (`KismetSystemLibrary.Delay` 2.0)
    (`|SpawnActorFromClass` "/Game/Assets/Blueprints/Points.Points_C" (`self.GetTransform`) "Undefined" "MultiplyWithRoot" null null)
    (`self.K2_DestroyActor`)))

(fn `UserConstructionScript`)