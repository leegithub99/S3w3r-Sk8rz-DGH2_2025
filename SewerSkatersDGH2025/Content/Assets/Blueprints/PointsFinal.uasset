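; PointsFinal is a collectible that adds one Cheese point to the skating third-person character.
; When a Player-tagged actor overlaps Scorez, it increments Cheese on player 0's character, hides itself, disables collision, plays a sound and destroys itself after a short delay.
; The pickup only runs when IsCollected is already true and then sets it true again, so the flag does not block repeat collection.
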(event `self.Scorez.OnComponentBeginOverlap`
  (params (OverlappedComponent :type "PrimitiveComponent Object Reference") (OtherActor :type "Actor Object Reference") (OtherComp :type "PrimitiveComponent Object Reference") (OtherBodyIndex :type Integer) (bFromSweep :type Boolean) (SweepResult :type "HitResult Structure (by ref)"))
  (if (`self.ActorHasTag` OtherActor "Player")
    (bind _asbp_third_person_character_skate (cast `/Game/Assets/Blueprints/BP_ThirdPersonCharacterSkate` (`GameplayStatics.GetPlayerCharacter` 0)))
    (if (`self.isCollected`)
      (set `self.isCollected` true)
      (set `/Game/Assets/Blueprints/BP_ThirdPersonCharacterSkate.Cheese` (+ (`/Game/Assets/Blueprints/BP_ThirdPersonCharacterSkate.Cheese` _asbp_third_person_character_skate) 1) _asbp_third_person_character_skate)
      (`self.SetActorHiddenInGame` true)
      (`self.SetActorEnableCollision` false)
      (`AudioComponent.Play` (`self.sfx`) 0.0)
      (`KismetSystemLibrary.Delay` 0.2)
      (`self.K2_DestroyActor`))))

(fn `UserConstructionScript`)