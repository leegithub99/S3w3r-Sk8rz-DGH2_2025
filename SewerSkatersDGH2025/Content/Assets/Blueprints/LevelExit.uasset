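; Level exit that stays hidden and without collision until the player has collected the required cheese, then loads the next level.
; Each Tick it casts the player to BP_SkateBoy and reveals itself with collision once Cheese exactly equals CheeseNeeded.
; A hit on its Cylinder by an actor tagged Player opens the level named in NextLevel.
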(event `self.ReceiveBeginPlay`
  (`self.SetActorHiddenInGame` true)
  (`self.SetActorEnableCollision` false))

(event `self.ReceiveTick`
  (params (DeltaSeconds :type "Float (single-precision)"))
  (bind _asbp_third_person_character_skate (cast `/Game/Assets/Blueprints/BP_SkateBoy` (`GameplayStatics.GetPlayerCharacter` 0)))
  (if (== (`/Game/Assets/Blueprints/BP_SkateBoy.Cheese` _asbp_third_person_character_skate) (`self.CheeseNeeded`))
    (`self.SetActorHiddenInGame` false)
    (`self.SetActorEnableCollision` true)))

(event `self.Cylinder.OnComponentHit`
  (params (HitComponent :type "PrimitiveComponent Object Reference") (OtherActor :type "Actor Object Reference") (OtherComp :type "PrimitiveComponent Object Reference") (NormalImpulse :type "Vector Structure") (Hit :type "HitResult Structure (by ref)"))
  (if (`self.ActorHasTag` OtherActor "Player")
    (`GameplayStatics.OpenLevel` (`self.nextLevel`))))

(fn `UserConstructionScript`)